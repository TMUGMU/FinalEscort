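; BP_Item is an item actor with a configurable mesh and an empty Pickup event.
; The construction script applies ItemMesh to the Mesh component.
; When player pawn 0 overlaps Box, a temporary fire emitter spawns at the mesh and replaces the InRangeParticles reference.
; The hide logic is bound to end overlap on InRangeParticles rather than Box, and each begin overlap spawns another emitter.
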(event `Pickup`)

(event `self.Box.OnComponentBeginOverlap`
  (params (OverlappedComponent :type "PrimitiveComponent Object Reference") (OtherActor :type "Actor Object Reference") (OtherComp :type "PrimitiveComponent Object Reference") (OtherBodyIndex :type Integer) (bFromSweep :type Boolean) (SweepResult :type "HitResult Structure (by ref)"))
  (if (== OtherActor (`GameplayStatics.GetPlayerPawn` 0))
    ;[1 1 1] temp stuff
    (bind _returnvalue (`GameplayStatics.SpawnEmitterAtLocation` "/Game/DefaultContent/StarterContent/Particles/P_Fire.P_Fire" (`SceneComponent.K2_GetComponentLocation` (`self.Mesh`))))
    (bind _output_get (set `self.InRangeParticles` _returnvalue))
    (`SceneComponent.SetVisibility` _output_get true false)))

(event `self.InRangeParticles.OnComponentEndOverlap`
  (params (OverlappedComponent :type "PrimitiveComponent Object Reference") (OtherActor :type "Actor Object Reference") (OtherComp :type "PrimitiveComponent Object Reference") (OtherBodyIndex :type Integer))
  (if (== OtherActor (`GameplayStatics.GetPlayerPawn` 0))
    ;[1 1 1] temp stuff
    (`SceneComponent.SetVisibility` (`self.InRangeParticles`) false false)))

(fn `UserConstructionScript`
  (`StaticMeshComponent.SetStaticMesh` (`self.Mesh`) (`self.ItemMesh`)))