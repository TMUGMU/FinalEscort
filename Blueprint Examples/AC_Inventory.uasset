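; AC_Inventory is an inventory component that tracks how many of each item is held.
; Items are stored in a map from item to amount, so AddItem either adds to an existing count or creates a new entry.
; PrintInventory loops over the map keys and prints each item's name and amount as text.
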(event `Add Item`
  (params (Item :type "/Game/1_MyAssets/Blueprints/BP_Item Class Reference") (Amount :type Integer))
  (if (`BlueprintMapLibrary.Map_Contains` (`self.Items`) Item)
    (`BlueprintMapLibrary.Map_Add` (`self.Items`) Item (+ (`BlueprintMapLibrary.Map_Find` (`self.Items`)) Amount))
    (else
      (`BlueprintMapLibrary.Map_Add` (`self.Items`) Item Amount))))

(fn `PrintInventory`
  (bind _keys (`BlueprintMapLibrary.Map_Keys` (`.Items` (`self.Items`))))
  (for _array_element _keys
    (`KismetSystemLibrary.PrintText` (`|FormatText` "{ItemName} | {Amount}" (`/Game/1_MyAssets/Blueprints/BP_Item.ItemName` _array_element) (`BlueprintMapLibrary.Map_Find` (`.Items` (`self.Items`)) _array_element)))))